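; EOBGame is a game flow actor that opens the party creation screen for a new game.
; NewGame adds a CreateParty widget to the viewport, clears InputVal and enables Tick to wait for input.
; Tick polls InputVal, stops itself once the value is positive, and calls NewGame again for option 1.
; BeginPlay calls Start, which is currently empty because its NewGame call is disconnected.
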(event `self.ReceiveBeginPlay`
  (`self.Start`))

(event `self.ReceiveTick`
  (params (DeltaSeconds :type "Float (single-precision)"))
  (if (`self.bWaitingForInput`)
    (if (> (`self.inputVal`) 0)
      (set `self.bWaitingForInput` false)
      (`self.SetActorTickEnabled` false)
      (switch `int` (`self.inputVal`)
        (:`1`
          (`self.NewGame`))))))

(fn `Input`
  (params (InputVal :type Integer))
  (set `self.inputVal` InputVal))

(fn `NewGame`
  (bind _returnvalue (`|CreateWidget` "/Game/Widgets/createParty.createParty_C"))
  (`UserWidget.AddToViewport` _returnvalue 0)
  (set `self.bWaitingForInput` true)
  (set `self.inputVal` 0)
  (`self.SetActorTickEnabled` true))

(fn `Start`)

(fn `UserConstructionScript`)